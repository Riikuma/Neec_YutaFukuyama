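; Garage actor with a single door and a pair of large gates that the player opens and closes with E.
; Two trigger volumes enable player input on any overlap and disable it on exit, setting a flag on entry to choose door or gates.
; E plays or reverses the selected Timeline based on its current value, driving mesh relative yaw, with the gate leaves on separate clockwise and counter-clockwise tracks.
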(event `self.Door_Trigger.OnComponentBeginOverlap`
  (params (OverlappedComponent :type "PrimitiveComponent Object Reference") (OtherActor :type "Actor Object Reference") (OtherComp :type "PrimitiveComponent Object Reference") (OtherBodyIndex :type Integer) (bFromSweep :type Boolean) (SweepResult :type "HitResult Structure (by ref)"))
  (`|ExecutionSequence`
    (:`then_0`
      ;[1 1 1] Differentiate trigger zones
      (set `self.isDoorTriggerActive` true))
    (:`then_1`
      (`self.EnableInput` (`GameplayStatics.GetPlayerController` 0) :!label _label))))

(event `self.Door_Trigger.OnComponentEndOverlap`
  (params (OverlappedComponent :type "PrimitiveComponent Object Reference") (OtherActor :type "Actor Object Reference") (OtherComp :type "PrimitiveComponent Object Reference") (OtherBodyIndex :type Integer))
  (`self.DisableInput` (`GameplayStatics.GetPlayerController` 0) :!label _label_2))

(event `self.Gates_Trigger.OnComponentBeginOverlap`
  (params (OverlappedComponent :type "PrimitiveComponent Object Reference") (OtherActor :type "Actor Object Reference") (OtherComp :type "PrimitiveComponent Object Reference") (OtherBodyIndex :type Integer) (bFromSweep :type Boolean) (SweepResult :type "HitResult Structure (by ref)"))
  (`|ExecutionSequence`
    (:`then_0`
      ;[1 1 1] Differentiate trigger zones
      (set `self.isDoorTriggerActive` false))
    (:`then_1`
      (goto _label))))

(event `Key|E`
  (params (Key :type "Key Structure"))
  (:`Pressed`
    (if (`self.isDoorTriggerActive`)
      ;[1 1 1] Door opening
      (if (< (stale _doorrot) 1.0)
        (bind (_direction _doorrot) (`Timeline|Door_Timeline` :!label _label_3)
          (:`Update`
            (`SceneComponent.K2_SetRelativeRotation` (`self.SM_Garage_Door`) (`KismetMathLibrary.MakeRotator` 0.0 0.0 _doorrot) false false)))
        (else
          (goto _label_3 :!via `Reverse`)))
      (else
        ;[1 1 1] Gates opening
        (if (< (stale _doorrot_ccw) 1.0)
          (bind (_direction_2 _doorrot_ccw _doorrot_cw) (`Timeline|Gate_Timeline` :!label _label_4)
            (:`Update`
              (`|ExecutionSequence`
                (:`then_0`
                  (`SceneComponent.K2_SetRelativeRotation` (`self.SM_Garage_Door_Large_02`) (`KismetMathLibrary.MakeRotator` 0.0 0.0 _doorrot_ccw) false false))
                (:`then_1`
                  (`SceneComponent.K2_SetRelativeRotation` (`self.SM_Garage_Door_Large_01`) (`KismetMathLibrary.MakeRotator` 0.0 0.0 _doorrot_cw) false false)))))
          (else
            (goto _label_4 :!via `Reverse`)))))))

(event `self.Gates_Trigger.OnComponentEndOverlap`
  (params (OverlappedComponent :type "PrimitiveComponent Object Reference") (OtherActor :type "Actor Object Reference") (OtherComp :type "PrimitiveComponent Object Reference") (OtherBodyIndex :type Integer))
  (goto _label_2))

(fn `UserConstructionScript`)